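; Trigger box Blueprint that benchmarks a nested-sum workload when the ThirdPersonCharacter overlaps its collision component.
; It timestamps the start, runs GetTotalSum on a C# component over NumberOfLoops, then prints elapsed milliseconds and the result.
; Equivalent Blueprint loop functions and a C++ TestPerformance call exist for comparison but are disconnected, so only the C# path runs.
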(event `self.CollisionComponent.OnComponentBeginOverlap`
  (params (OverlappedComponent :type "PrimitiveComponent Object Reference") (OtherActor :type "Actor Object Reference") (OtherComp :type "PrimitiveComponent Object Reference") (OtherBodyIndex :type Integer) (bFromSweep :type Boolean) (SweepResult :type "HitResult Structure (by ref)"))
  (cast `/Game/ThirdPersonCPP/Blueprints/ThirdPersonCharacter` OtherActor)
  (set `self.MyTime` (`KismetMathLibrary.Now`))
  ;[1 1 1] C Sharp
  (bind _returnvalue (`CSharpPerformanceTestComponent.GetTotalSum` (`self.CSharpPerformanceTestComponentBP`) (`KismetMathLibrary.Conv_IntToDouble` (`self.NumberOfLoops`))))
  (`self.PrintPerformanceValues` _returnvalue))

(fn `GetTotalSumBlueprints`
  (params (NumberOfLoops :type Integer))
  (returns (MyTotalValue :type "Float (double-precision)"))
  (locals (MyResult :type "Float (double-precision)"))
  (for _index (range 1 (+ NumberOfLoops 1))
    (bind _myresult (`self.SumNBlueprints` (`KismetMathLibrary.Conv_IntToDouble` _index)))
    (set `local.MyResult` (+ _myresult (`local.MyResult`))))
  (return (`local.MyResult`)))

(fn `PrintPerformanceValues`
  (params (PerfResults :type "Float (double-precision)"))
  (`KismetSystemLibrary.PrintString` (`KismetStringLibrary.Concat_StrStr` (`KismetStringLibrary.Conv_DoubleToString` (`KismetMathLibrary.GetTotalMilliseconds` (- (`KismetMathLibrary.Now`) (`self.MyTime`)))) " ms - result: " (`KismetStringLibrary.Conv_DoubleToString` PerfResults))))

(fn `SumNBlueprints`
  (params (N :type "Float (double-precision)"))
  (returns (MyResult :type "Float (double-precision)"))
  (locals (Temp :type "Float (double-precision)"))
  (for _index (range 1 (+ (`KismetMathLibrary.FTrunc` N) 1))
    (set `local.Temp` (+ (`KismetMathLibrary.Conv_IntToDouble` _index) (`local.Temp`))))
  (return (`local.Temp`)))

(fn `UserConstructionScript`)